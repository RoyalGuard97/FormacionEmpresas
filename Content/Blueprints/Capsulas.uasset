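; Capsulas is a destructible capsule actor that takes damage only from weapons matching its color weakness and spawns another actor when destroyed.
; AnyDamage casts the damage type to ProjectileDamage and lowers Health only when its WeaponColor equals Weakness.
; A surviving hit plays a damage sound, while zero health destroys the capsule.
; The Destroyed event then spawns the class in ClaseASpawnear at the capsule's location.
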(event `self.ReceiveAnyDamage`
  (params (Damage :type "Float (single-precision)") (DamageType :type "DamageType Object Reference") (InstigatedBy :type "Controller Object Reference") (DamageCauser :type "Actor Object Reference"))
  (bind _health (`self.Health`))
  (bind _asprojectile_damage (cast `/Game/Weapons/Projectiles/Damage/ProjectileDamage` DamageType))
  (if (`|EnumEquality` (`self.Weakness`) (`/Game/Weapons/Projectiles/Damage/ProjectileDamage.Weapon Color` _asprojectile_damage))
    (set `self.Health` (- _health Damage))
    (if (<= _health 0.0)
      (`self.K2_DestroyActor`)
      (else
        (`GameplayStatics.PlaySound2D` "/Game/Sonido/Damage.Damage" 1.0 1.0 0.0 null null)))))

(event `self.ReceiveDestroyed`
  (bind _returnvalue_location (`KismetMathLibrary.BreakTransform` (`self.GetTransform`)))
  (`|SpawnActorFromClass` (`self.ClaseASpawnear`) (`KismetMathLibrary.Conv_VectorToTransform` _returnvalue_location) "Undefined" "OverrideRootScale" null null))

(fn `UserConstructionScript`)