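; Enemy spawner that creates RedEnemy actors at random points inside its SpawnVolumen box.
; The SpawnEnemy event spawns one enemy only while the live RedEnemy count is below MaxEnemies and the running spawn counter is under its hardcoded cap.
; Each new enemy receives fixed movement speed, damage and health values.
; Nothing in this graph calls SpawnEnemy, and Tick is unused.
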(event `SpawnEnemy`
  (bind _spawnvolumen (`self.SpawnVolumen`))
  (bind _outactors (`GameplayStatics.GetAllActorsOfClass` "/Game/Enemies/Blueprints/RedEnemy.RedEnemy_C"))
  (if (and (< (`KismetArrayLibrary.Array_Length` _outactors) (`self.MaxEnemies`)) (<= (`self.Contador de Enemigos`) 19))
    (`/Engine/EditorBlueprintResources/StandardMacros.IncrementInt` (`self.Contador de Enemigos`)
      (:`  `
        (bind _returnvalue (`|SpawnActorFromClass` "/Game/Enemies/Blueprints/RedEnemy.RedEnemy_C" (`KismetMathLibrary.Conv_VectorToTransform` (`KismetMathLibrary.RandomPointInBoundingBox` (`SceneComponent.K2_GetComponentLocation` _spawnvolumen) (`BoxComponent.GetScaledBoxExtent` _spawnvolumen))) "Undefined" "OverrideRootScale" null (struct :`R` 1.0 :`G` 0.005134 :`A` 1.0) null))
        (set `/Game/Enemies/Blueprints/BP_MasterEnemy.Enemy Movement Speed` 550.0 _returnvalue)
        (set `/Game/Enemies/Blueprints/BP_MasterEnemy.DañoProvocado` 10.0 _returnvalue)
        (set `/Game/Enemies/Blueprints/BP_MasterEnemy.Health` 10.0 _returnvalue)))))

(fn `UserConstructionScript`)